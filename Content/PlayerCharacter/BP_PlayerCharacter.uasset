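; Player character Blueprint that sets up locomotion animation, grants dodge-roll and equip-item abilities, and manages stamina regeneration.
; The Ability System Component comes from the PlayerState; BeginPlay also links the anim layer and sends an event equipping Unarmed in the left slot.
; An attribute-change listener applies a regen-delay effect when stamina drops, and removes tagged regen effects on a drop or upon reaching max.
; Q activates the dodge by stored spec handle, and E toggles stance.
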(event `self.ReceiveBeginPlay`
  (bind _returnvalue (`AbilitySystemBlueprintLibrary.GetAbilitySystemComponent` (`self.GetAPSPlayerState`)))
  (`SkeletalMeshComponent.LinkAnimClassLayers` (`self.Mesh`) "/Game/PlayerCharacter/Animation/ABP_Locomotion.ABP_Locomotion_C")
  ;[0.7969 0 0 0.5] Adding Abilities should be moved to a dedicated location with ability sets, possibly a subsystem.
  (bind _returnvalue_2 (`AbilitySystemComponent.K2_GiveAbility` _returnvalue "/Game/GameplayAbilitySystem/GA_DodgeRoll.GA_DodgeRoll_C" 0 -1))
  (set `self.DodgeAbilitySpecHandle` _returnvalue_2)
  (`AbilitySystemComponent.K2_GiveAbility` _returnvalue "/Game/GameplayAbilitySystem/GA_EquipItem.GA_EquipItem_C" 0 -1)
  (bind (_asynctaskproxy _attribute _newvalue _oldvalue) (`AbilityAsync_WaitAttributeChanged.WaitForAttributeChanged` null (struct :`AttributeName` "Stamina" :`Attribute` "/Script/AnimationPlaySpace.BasicAttributeSet:Stamina" :`AttributeOwner` "/Script/CoreUObject.Class'/Script/AnimationPlaySpace.BasicAttributeSet'"))
    (:`then`
      (`AbilitySystemBlueprintLibrary.SendGameplayEventToActor` self (struct :`TagName` "Event.EquipItem") (make `GameplayEventData` :`OptionalObject` "/Game/Data/WeaponData/DA_Unarmed.DA_Unarmed" :`TargetTags` (struct :`GameplayTags` (struct :`(TagName` "Equipment.Slot.Left"))))))
    (:`Changed`
      (`self.HandleStaminaChanged` _newvalue _oldvalue))))

(event `self.ReceiveTick`
  (params (DeltaSeconds :type "Float (single-precision)")))

(event `Key|Q`
  (params (Key :type "Key Structure"))
  (:`Pressed`
    (`AbilitySystemComponent.TryActivateAbility` (`AbilitySystemBlueprintLibrary.GetAbilitySystemComponent` (`self.GetAPSPlayerState`)) (`self.DodgeAbilitySpecHandle`) true)))

(event `HandleStaminaChanged`
  (params (newValue :type "Float (double-precision)") (oldValue :type "Float (double-precision)"))
  (bind _returnvalue (`AbilitySystemBlueprintLibrary.GetAbilitySystemComponent` (`self.GetAPSPlayerState`)))
  (bind _staminamax_basevalue (break `GameplayAttributeData` (`BasicAttributeSet.StaminaMax` (`APSPlayerState.BasicAttributeSet` (`self.GetAPSPlayerState`)))))
  (if (< newValue oldValue)
    (`AbilitySystemComponent.BP_ApplyGameplayEffectToSelf` :`self` _returnvalue :`GameplayEffectClass` "/Game/GameplayAbilitySystem/GameplayEffects/GE_Satus_StaminaRegen_Delay.GE_Satus_StaminaRegen_Delay_C")
    (`AbilitySystemComponent.RemoveActiveEffectsWithGrantedTags` _returnvalue (struct :`GameplayTags` (struct :`(TagName` "Status.Stamina.Regen"))) :!label _label)
    (elif (>= newValue _staminamax_basevalue)
      (goto _label))))

(event `Key|E`
  (params (Key :type "Key Structure"))
  (:`Pressed`
    (`self.SetStance` (not (`self.GetStance`)))))

(fn `UserConstructionScript`)